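; Tank Blueprint that registers its gun and handles player aiming input.
; On BeginPlay it passes the TankGun component to SetBarrelReference.
; The azimuth axis yaws an AzimuthGimbal and the elevation axis pitches the SpringArm, keeping the two rotations on separate components.
; Both use local rotations scaled by world delta seconds and a fixed speed, so turn rate is frame-rate independent.
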(event EventBeginPlay
  (Class|Tank|SetBarrelReference (Variables|Default|GetTankGun)))

(event Input|AxisEvents|InputAxisAimingAzimuth
  (params (AxisValue :type Float%20%28single-precision%29))
  (Transformation|AddLocalRotation (Variables|Default|GetAzimuth%20Gimbal) (Math|Rotator|MakeRotator 0.0 0.0 (* AxisValue (Utilities|Time|GetWorldDeltaSeconds) 5e+01)) false false))

(event Input|AxisEvents|InputAxisAimingElevation
  (params (AxisValue :type Float%20%28single-precision%29))
  (Transformation|AddLocalRotation (Variables|Default|GetSpringArm) (Math|Rotator|MakeRotator 0.0 (* AxisValue (Utilities|Time|GetWorldDeltaSeconds) 5e+01) 0.0) false false))

(fn ConstructionScript)